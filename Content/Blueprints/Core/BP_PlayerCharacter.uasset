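; Player character Blueprint that handles movement and look input through axis events.
; Forward and strafe movement follow control-rotation yaw only, keeping movement independent of pitch.
; LookRight turns controller yaw, while LookUp pitches the CameraRoot component locally without clamping.
; Strafing sets IsStrafing and stores a direction rotator from the right vector, negating the rotator itself for leftward input, before applying movement.
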(event EventBeginPlay)

(event EventActorBeginOverlap
  (params (OtherActor :type Actor%20Object%20Reference)))

(event EventTick
  (params (DeltaSeconds :type Float%20%28single-precision%29)))

(event Input|AxisEvents|InputAxisLookRight
  (params (AxisValue :type Float%20%28single-precision%29))
  (Pawn|Input|AddControllerYawInput AxisValue))

(event Input|AxisEvents|InputAxisLookUp
  (params (AxisValue :type Float%20%28single-precision%29))
  (Transformation|AddLocalRotation (Variables|Default|GetCameraRoot) (Math|Rotator|MakeRotator 0.0 AxisValue 0.0) false false))

(event Input|AxisEvents|InputAxisMoveForward
  (params (AxisValue :type Float%20%28single-precision%29))
  (Pawn|Input|AddMovementInput (Math|Vector|GetForwardVector (Math|Rotator|MakeRotator 0.0 0.0 (.Yaw (Math|Rotator|BreakRotator (Pawn|GetControlRotation :!class /Script/Engine.Pawn))))) AxisValue false))

(event Input|AxisEvents|InputAxisStrafeRight
  (params (AxisValue :type Float%20%28single-precision%29))
  (bind _returnvalue (Pawn|GetControlRotation :!class /Script/Engine.Pawn))
  (bind _yaw (Math|Rotator|BreakRotator _returnvalue))
  (bind _returnvalue_2 (Math|Rotator|MakeRotator 0.0 0.0 _yaw))
  (bind _returnvalue_3 (Math|Vector|GetRightVector _returnvalue_2))
  (bind _output_get (Variables|Default|SetIsStrafing (!= AxisValue 0.0)))
  (if _output_get
    (CallFunction|Strafe _returnvalue_3 AxisValue _returnvalue_3)))

(fn ConstructionScript)

(fn Strafe
  (params (WorldDirection :type Vector) (ScaleValue :type Float%20%28single-precision%29) (InVec :type Vector))
  (bind _returnvalue (Math|Conversions|RotationFromXVector InVec))
  (if (> ScaleValue 0.0)
    (Variables|Default|SetStrafeDiretion _returnvalue)
    (else
      (Variables|Default|SetStrafeDiretion (* _returnvalue -1.0))))
  (Pawn|Input|AddMovementInput WorldDirection ScaleValue false)
  (return))